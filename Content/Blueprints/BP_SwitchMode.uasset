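; BP_SwitchMode is the mode-selection actor that lets the player become a Prop, Hunter or Spectator.
; On BeginPlay it shows the cursor and opens WG_ChooseMode, passing itself as PlayerRef.
; SwitchmodeRunOnServer clears the widgets, hides the cursor, then spawns the matching pawn at a fixed location and possesses it with player controller 0.
; Spectator currently spawns BP_HunterPlayer, and SwitchModeMulticast is an empty stub.
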(event Custom|SwitchmodeRunOnServer
  (params (Selection :type E_GameMode%20Enum :default "NewEnumerator0"))
  (Viewport|RemoveAllWidgets)
  (Variables|/Script/Engine.PlayerController|SetbShowMouseCursor (Game|GetPlayerController 0) false)
  (switch Utilities|FlowControl|Switch|SwitchonE_GameMode Selection
    (:NewEnumerator0
      (bind _returnvalue (Game|SpawnActorfromClass "/Game/Blueprints/PropBP/BP_PropPlayer.BP_PropPlayer_C" (Math|Transform|MakeTransform "640.000000,910.000000,92.012604" "0, 0, 0" "1.000000,1.000000,1.000000") "Undefined" 0 0))
      (Pawn|Possess (Game|GetPlayerController 0) _returnvalue))
    (:NewEnumerator1
      (bind _returnvalue_2 (Game|SpawnActorfromClass "/Game/Blueprints/HunterBP/BP_HunterPlayer.BP_HunterPlayer_C" (Math|Transform|MakeTransform "640.000000,910.000000,92.012604" "0, 0, 0" "1.000000,1.000000,1.000000") "Undefined" 0 0))
      (Pawn|Possess (Game|GetPlayerController 0) _returnvalue_2))
    (:NewEnumerator2
      (bind _returnvalue_3 (Game|SpawnActorfromClass "/Game/Blueprints/HunterBP/BP_HunterPlayer.BP_HunterPlayer_C" (Math|Transform|MakeTransform "640.000000,910.000000,92.012604" "0, 0, 0" "1.000000,1.000000,1.000000") "Undefined" 0 0))
      (Pawn|Possess (Game|GetPlayerController 0) _returnvalue_3))))

(event Custom|SwitchModeMulticast
  (params (Selection :type E_GameMode%20Enum :default "NewEnumerator0")))

(event EventBeginPlay
  (Variables|/Script/Engine.PlayerController|SetbShowMouseCursor (Game|GetPlayerController 0) true)
  (bind _returnvalue (UserInterface|CreateWidget "/Game/Widgets/WG_ChooseMode.WG_ChooseMode_C" 0 self))
  (UserInterface|Viewport|AddtoViewport _returnvalue 0))

(fn ConstructionScript)