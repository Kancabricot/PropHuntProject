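; Custom game instance that handles LAN multiplayer sessions: creating, finding and joining them.
; Creating a session succeeds by opening a level as a listen server.
; Searching requests a single result, stores it, then tells the main menu to show the list, or to reset its join state when the search is empty or fails.
; Joining takes a chosen search result and only prints success or failure.
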(event Custom|Event_JoinSession
  (params (PlayerController :type Player%20Controller%20Object%20Reference) (SessionToJoin :type Blueprint%20Session%20Result%20Structure%20%28by%20ref%29))
  (|JoinSession PlayerController SessionToJoin
    (:OnSuccess
      (Development|PrintString "Join Success"))
    (:OnFailure
      (Development|PrintString "Join Fail"))))

(event Custom|Event_CreateSession
  (params (PlayerController :type Player%20Controller%20Object%20Reference))
  (|Session PlayerController 40 true
    (:OnSuccess
      (Development|PrintString "Creation Success")
      (Game|OpenLevel(byObjectReference) (Variables|Default|GetLevel) true "listen"))
    (:OnFailure
      (Development|PrintString "Fail Creation"))))

(event Custom|Event_FindSession
  (params (PlayerController :type Player%20Controller%20Object%20Reference) (MainMenuRef :type WG%20Main%20Menu%20Object%20Reference))
  (bind _results (|FindSessions PlayerController 1 true)
    (:OnSuccess
      (bind _output_get (Variables|Default|SetSessionsResults _results))
      (if (Utilities|Array|IsNotEmpty _output_get)
        (Default|EventShowList MainMenuRef)
        (else
          (Default|EventResetJoin MainMenuRef :!label _label))))
    (:OnFailure
      (Development|PrintString "Fail Find")
      (goto _label))))